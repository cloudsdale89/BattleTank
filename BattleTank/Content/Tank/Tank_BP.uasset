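; Tank Blueprint that handles player camera aiming and firing input.
; On BeginPlay it passes its Turret and Barrel components to setter functions whose logic is not in these graphs.
; Azimuth input yaws an azimuth gimbal and elevation input pitches the spring arm, separating the two rotation axes.
; The Fire action calls a Fire function, also defined outside these graphs.
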(event `self.ReceiveBeginPlay`
  (`self.SetTurretReference` (`self.Turret`))
  (`self.SetBarrelReference` (`self.Barrel`)))

(event `InputAxis|AimAzimuth`
  (params (AxisValue :type "Float (single-precision)"))
  ;[1 1 1] Input Binding
  (`SceneComponent.K2_AddLocalRotation` (`self.Azimuth Gimbal`) (`KismetMathLibrary.MakeRotator` 0.0 0.0 AxisValue) false false))

(event `InputAxis|AimElevation`
  (params (AxisValue :type "Float (single-precision)"))
  ;[1 1 1] Input Binding
  (`SceneComponent.K2_AddLocalRotation` (`self.SpringArm`) (`KismetMathLibrary.MakeRotator` 0.0 AxisValue) false false))

(event `InputAction|Fire`
  (params (Key :type "Key Structure"))
  ;[1 1 1] Input Binding
  (:`Pressed`
    (`self.Fire`)))

(fn `UserConstructionScript`)